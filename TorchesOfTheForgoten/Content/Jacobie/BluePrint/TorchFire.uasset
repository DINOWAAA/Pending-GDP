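; TorchFire is a torch light that burns down over time and kills the player when it gets too dim.
; The firelight starts at maximum intensity, then Tick slowly interpolates it toward the minimum with FInterpTo and prints it for debugging.
; At or below the killing threshold, Tick finds the first-person characters and calls HandlePlayerDeath after a short Delay.
; A Timeline node is present but never runs.
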(event `self.ReceiveBeginPlay`
  (`LightComponent.SetIntensity` (`self.FirelightComponent`) (`self.Max Light Intensity`)))

(event `self.ReceiveTick`
  (params (DeltaSeconds :type "Float (single-precision)"))
  (bind _intensity (`LightComponentBase.Intensity` (`self.FirelightComponent`)))
  (`KismetSystemLibrary.PrintString` (`KismetStringLibrary.Conv_DoubleToString` _intensity))
  (bind _output_get (set `self.Current Light Intensity` (`KismetMathLibrary.FInterpTo` _intensity (`self.Min Light Intensity`) DeltaSeconds 0.1)))
  (`LightComponent.SetIntensity` (`self.FirelightComponent`) _output_get)
  (if (<= (`LightComponentBase.Intensity` (`self.FirelightComponent`)) (`self.Killing light intensity`))
    (bind _outactors (`GameplayStatics.GetAllActorsOfClass` "/Game/FirstPerson/Blueprints/BP_FirstPersonCharacter.BP_FirstPersonCharacter_C"))
    (`KismetSystemLibrary.Delay` 1.0)
    (`/Game/FirstPerson/Blueprints/BP_FirstPersonCharacter.Handle Player Death` _outactors)))

(fn `UserConstructionScript`)